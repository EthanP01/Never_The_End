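; Magic ball projectile that starts attached, is thrown along a given direction and speed, and bursts on contact.
; ThrowProjectile detaches it, sets the projectile movement velocity, then fades MagicFX and shortens the actor's lifespan after a delay.
; Sphere overlap with anything but the player spawns a Niagara chaos explosion and destroys the ball, applying no damage.
; A BeginPlay lifespan caps its lifetime, and DestroyProjectile provides early cleanup.
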(event `self.ReceiveBeginPlay`
  (`self.SetLifeSpan` 15.0))

(event `ThrowProjectile`
  (params (Direction :type "Vector Structure") (Speed :type "Float (double-precision)"))
  (`self.K2_DetachFromActor` "KeepWorld" "KeepWorld" "KeepWorld")
  (set `MovementComponent.Velocity` (* Direction Speed) (`self.ProjectileMovement`))
  (`KismetSystemLibrary.Delay` (`self.BallLifespan`))
  (`ActorComponent.Deactivate` (`self.Magic FX`))
  (`self.SetLifeSpan` 1.0))

(event `Destroy Projectile`
  (`ActorComponent.Deactivate` (`self.Magic FX`))
  (`self.SetLifeSpan` 0.1))

(event `self.Sphere.OnComponentBeginOverlap`
  (params (OverlappedComponent :type "PrimitiveComponent Object Reference") (OtherActor :type "Actor Object Reference") (OtherComp :type "PrimitiveComponent Object Reference") (OtherBodyIndex :type Integer) (bFromSweep :type Boolean) (SweepResult :type "HitResult Structure (by ref)"))
  (if (!= OtherActor (`GameplayStatics.GetPlayerCharacter` 0))
    (`KismetSystemLibrary.PrintString` (`KismetStringLibrary.Concat_StrStr` "Hit || " (`KismetSystemLibrary.GetDisplayName` OtherActor)))
    (`NiagaraFunctionLibrary.SpawnSystemAtLocation` "/Game/FX/NS_ChaosExplosion.NS_ChaosExplosion" (`SceneComponent.K2_GetComponentLocation` (`self.Magic FX`)))
    (`self.K2_DestroyActor`)))

(fn `UserConstructionScript`)