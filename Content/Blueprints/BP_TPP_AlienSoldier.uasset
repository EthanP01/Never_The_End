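; Player character Blueprint for an alien soldier, apparently third-person, handling movement, camera and aim input.
; Movement follows control-rotation yaw, and look input drives controller yaw and pitch with optional Y inversion.
; Sprint and walk-toggle inputs switch max walk speed between unarmed walk, run and sprint values, with run set at BeginPlay when unarmed.
; Jump uses built-in Character functions, while ADS only sets an Aiming flag.
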(event `self.ReceiveBeginPlay`
  (`|ExecutionSequence`
    (:`then_1`
      (if (not (`self.Armed`))
        (set `CharacterMovementComponent.MaxWalkSpeed` (`self.UnarmedRunSpeed`) (`self.CharacterMovement`))))))

(event `self.ReceiveTick`
  (params (DeltaSeconds :type "Float (single-precision)")))

(event `InputAxis|MoveForward`
  (params (AxisValue :type "Float (single-precision)"))
  (bind (_returnvalue_roll _returnvalue_pitch _returnvalue_yaw) (`KismetMathLibrary.BreakRotator` (`self.GetControlRotation`)))
  ;[0 0 0] Walking
  (`self.AddMovementInput` (`KismetMathLibrary.GetForwardVector` (`KismetMathLibrary.MakeRotator` 0.0 0.0 _returnvalue_yaw)) AxisValue))

(event `InputAxis|LookX`
  (params (AxisValue :type "Float (single-precision)"))
  ;[0 0 0] Camera Controls
  (`self.AddControllerYawInput` AxisValue))

(event `InputAxis|LookY`
  (params (AxisValue :type "Float (single-precision)"))
  ;[0 0 0] Camera Controls
  (if (`self.InvertYLook`)
    (`self.AddControllerPitchInput` AxisValue)
    (else
      (`self.AddControllerPitchInput` (* AxisValue -1.0)))))

(event `InputAxis|Strafe`
  (params (AxisValue :type "Float (single-precision)"))
  (bind (_returnvalue_roll _returnvalue_pitch _returnvalue_yaw) (`KismetMathLibrary.BreakRotator` (`self.GetControlRotation`)))
  ;[0 0 0] Walking
  (`self.AddMovementInput` (`KismetMathLibrary.GetRightVector` (`KismetMathLibrary.MakeRotator` 0.0 0.0 _returnvalue_yaw)) AxisValue))

(event `InputAction|Sprint`
  (params (Key :type "Key Structure"))
  (bind _charactermovement (`self.CharacterMovement`))
  ;[0 0 0] Sprinting
  (:`Pressed`
    (set `CharacterMovementComponent.MaxWalkSpeed` (`self.UnarmedSprintSpeed`) _charactermovement)
    (set `self.Walking` false))
  (:`Released`
    (set `CharacterMovementComponent.MaxWalkSpeed` (`self.UnarmedRunSpeed`) _charactermovement)))

(event `InputAction|Toggle Walk`
  (params (Key :type "Key Structure"))
  (bind _charactermovement (`self.CharacterMovement`))
  (bind _walking (`self.Walking`))
  ;[0 0 0] Toggle Walk
  (:`Pressed`
    (if _walking
      (set `CharacterMovementComponent.MaxWalkSpeed` (`self.UnarmedRunSpeed`) _charactermovement)
      (else
        (set `CharacterMovementComponent.MaxWalkSpeed` (`self.UnarmedWalkSpeed`) _charactermovement)))
    (set `self.Walking` (not _walking))))

(event `InputAction|Jump`
  (params (Key :type "Key Structure"))
  ;[0 0 0] Jumping
  (:`Pressed`
    (`self.Jump`))
  (:`Released`
    (`self.StopJumping`)))

(event `InputAction|ADS`
  (params (Key :type "Key Structure"))
  (:`Pressed`
    (set `self.Aiming` true))
  (:`Released`
    (set `self.Aiming` false)))

(fn `UserConstructionScript`)