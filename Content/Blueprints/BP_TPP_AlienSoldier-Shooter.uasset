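; Third-person alien soldier player character that moves, jumps and fights with thrown chaos-ball magic and a spawnable shield area.
; Walk, sprint and charge (aim) states feed SetSpeed, which selects the max walk speed.
; Charge or attack spawns a ball on the right-hand socket, and the attack montage's notify throws it along the camera's forward vector.
; Montage notifies and callbacks also time jumping, landing and attack resets.
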(event `self.ReceiveBeginPlay`
  (`|ExecutionSequence`
    (:`then_0`
      (`self.SetSpeed`))))

(event `self.ReceiveTick`
  (params (DeltaSeconds :type "Float (single-precision)")))

(event `InputAxis|MoveForward`
  (params (AxisValue :type "Float (single-precision)"))
  (bind (_returnvalue_roll _returnvalue_pitch _returnvalue_yaw) (`KismetMathLibrary.BreakRotator` (`self.GetControlRotation`)))
  ;[0 0 0] Walking
  (`self.AddMovementInput` (`KismetMathLibrary.GetForwardVector` (`KismetMathLibrary.MakeRotator` 0.0 0.0 _returnvalue_yaw)) AxisValue))

(event `InputAxis|LookX`
  (params (AxisValue :type "Float (single-precision)"))
  ;[0 0 0] Camera Controls
  (`self.AddControllerYawInput` AxisValue))

(event `InputAxis|LookY`
  (params (AxisValue :type "Float (single-precision)"))
  ;[0 0 0] Camera Controls
  (if (`self.InvertYLook`)
    (`self.AddControllerPitchInput` AxisValue)
    (else
      (`self.AddControllerPitchInput` (* AxisValue -1.0)))))

(event `InputAxis|Strafe`
  (params (AxisValue :type "Float (single-precision)"))
  (bind (_returnvalue_roll _returnvalue_pitch _returnvalue_yaw) (`KismetMathLibrary.BreakRotator` (`self.GetControlRotation`)))
  ;[0 0 0] Walking
  (`self.AddMovementInput` (`KismetMathLibrary.GetRightVector` (`KismetMathLibrary.MakeRotator` 0.0 0.0 _returnvalue_yaw)) AxisValue))

(event `InputAction|Sprint`
  (params (Key :type "Key Structure"))
  ;[0 0 0] Sprinting
  (:`Pressed`
    (set `self.Sprinting` true)
    (set `self.Walking` false)
    (`self.SetSpeed` :!label _label))
  (:`Released`
    (set `self.Sprinting` false)
    (goto _label)))

(event `InputAction|Toggle Walk`
  (params (Key :type "Key Structure"))
  ;[0 0 0] Toggle Walk
  (:`Pressed`
    (set `self.Walking` (not (`self.Walking`)))
    (`self.SetSpeed`)))

(event `InputAction|Jump`
  (params (Key :type "Key Structure"))
  (bind _mesh (`self.Mesh`))
  ;[0 0 0] Jumping
  (:`Pressed`
    (if (not (`self.Jumping`))
      (`|PlayMontage` _mesh "/Game/Characters/AlienSoldier/Animations/AM_Jumping_Up.AM_Jumping_Up" 1.0 0.3
        (:`then`
          (set `self.Jumping` true))
        (:`OnCompleted`
          (if (`NavMovementComponent.IsFalling` (`self.CharacterMovement`))
            (`|PlayMontage` _mesh "/Game/Characters/AlienSoldier/Animations/AM_Falling_Idle.AM_Falling_Idle")))
        (:`OnNotifyBegin`
          (`self.Jump`)))))
  (:`Released`
    (`self.StopJumping`)))

(event `self.OnLanded`
  (params (Hit :type "HitResult Structure (by ref)"))
  (`self.StopAnimMontage` "/Game/Characters/AlienSoldier/Animations/AM_Falling_Idle.AM_Falling_Idle")
  (`|PlayMontage` (`self.Mesh`) "/Game/Characters/AlienSoldier/Animations/AM_Falling_To_Landing.AM_Falling_To_Landing" 1.0 0.2
    (:`OnInterrupted`
      _)
    (:`OnNotifyBegin`
      _))
  (set `self.Jumping` false))

(event `InputAction|ShieldAbility`
  (params (Key :type "Key Structure"))
  ;[0 0 0] Chaos Shield Area
  (:`Pressed`
    (if (not (`self.SpawnedShield`))
      (set `self.SpawnedShield` true)
      (bind _returnvalue (`|SpawnActorFromClass` "/Game/Blueprints/BP_ChaosShieldArea.BP_ChaosShieldArea_C" (`self.GetTransform`) "Undefined" "OverrideRootScale" null null))
      (`/Game/Blueprints/BP_ChaosShieldArea.Spawned` _returnvalue))))

(event `InputAction|Charge`
  (params (Key :type "Key Structure"))
  (bind _chaosball (`self.ChaosBall`))
  ;[0 0 0] Charge
  (:`Pressed`
    (if (not (`self.Attacking`))
      (set `self.Charging` true)
      (set `self.bUseControllerRotationYaw` true)
      (`self.SetSpeed`)
      (bind _returnvalue (`|SpawnActorFromClass` "/Game/Blueprints/BP_ChaosBall.BP_ChaosBall_C" (`SceneComponent.K2_GetComponentToWorld` (`self.RH_Magic Socket`)) "Undefined" "OverrideRootScale" null null))
      (`self.K2_AttachToComponent` _returnvalue (`self.Mesh`) "R_Hand_MagicSocket" "KeepWorld" "KeepWorld" "KeepWorld" true)
      (bind _output_get (set `self.ChaosBall` _returnvalue))
      (set `self.CurrentMagicAbility` _output_get)))
  (:`Released`
    (set `self.Charging` false)
    (set `self.bUseControllerRotationYaw` false)
    (`self.SetSpeed`)
    (if (not (`self.Attacking`))
      (`/Engine/EditorBlueprintResources/StandardMacros.IsValid` _chaosball
        (:`Is Valid`
          (`/Game/Blueprints/BP_ChaosBall.Destroy Projectile` _chaosball)
          (set `self.bUseControllerRotationYaw` false))))))

(event `InputAction|Attack`
  (params (Key :type "Key Structure"))
  (bind _mesh (`self.Mesh`))
  (bind _chaosball (`self.ChaosBall`))
  (bind _projectilespeed (`self.ProjectileSpeed`))
  (bind _returnvalue (`SceneComponent.GetForwardVector` (`self.Camera`)))
  ;[0 0 0] Attack
  (:`Pressed`
    (if (not (`self.Attacking`))
      (set `self.Attacking` true)
      (`/Engine/EditorBlueprintResources/StandardMacros.IsValid` (`self.ChaosBall`)
        (:`Is Valid`
          _)
        (:`Is Not Valid`
          (`self.SpawnAbility` (`SceneComponent.K2_GetComponentToWorld` (`self.RH_Magic Socket`)) (`self.Mesh`) "R_Hand_MagicSocket" (`self.ProjectileEquipped?`))))
      (if (`self.Charging`)
        (`|PlayMontage` _mesh "/Game/Characters/AlienSoldier/Animations/Mage/AM_Standing_1H_MagicAttack_01.AM_Standing_1H_MagicAttack_01"
          (:`then`
            (set `self.bUseControllerRotationYaw` true))
          (:`OnCompleted`
            (set `self.Attacking` false)
            (if (`self.Charging`)
              (`self.SpawnAbility` (`SceneComponent.K2_GetComponentToWorld` (`self.RH_Magic Socket`)) (`self.Mesh`) "R_Hand_MagicSocket" (`self.ProjectileEquipped?`))))
          (:`OnInterrupted`
            (set `self.Attacking` false))
          (:`OnNotifyBegin`
            (`/Game/Blueprints/BP_ChaosBall.ThrowProjectile` _chaosball _returnvalue _projectilespeed)
            (set `self.ChaosBall` null)))
        (else
          (`|PlayMontage` _mesh "/Game/Characters/AlienSoldier/Animations/Mage/AM_Standing_1H_MagicAttack_01.AM_Standing_1H_MagicAttack_01" 1.5
            (:`then`
              (set `self.bUseControllerRotationYaw` true))
            (:`OnCompleted`
              (set `self.Attacking` false :!label _label)
              (set `self.bUseControllerRotationYaw` false)
              (set `self.ChaosBall` null))
            (:`OnInterrupted`
              (goto _label))
            (:`OnNotifyBegin`
              (`/Game/Blueprints/BP_ChaosBall.ThrowProjectile` _chaosball _returnvalue _projectilespeed))))))))

(fn `UserConstructionScript`)